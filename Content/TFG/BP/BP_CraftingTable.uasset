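; Crafting table puzzle that tracks whether pieces are attached to their matching left, right and center anchors.
; Anchor events matching ConnectorID update PiezasCorrectas and run ComprobarPieza; center detach also writes true, and fake anchors do nothing.
; At twelve map entries, regardless of value, it changes the GameState phase.
; Otherwise, after a delay, it shows or hides each AnchorToMeshMap actor by its flag.
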(event `self.ReceiveBeginPlay`
  (bind `_asbp_oña_game_state_base` (cast `/Game/TFG/BP/BP_Oña_GameStateBase` (`GameplayStatics.GetGameState`)))
  (set `self.As BP Oña Game State Base` `_asbp_oña_game_state_base`))

(event `self.Anchor_5L_1.ActorGotDetached`
  (params (Anchor :type "/XRAIlab/Blueprints/Components/Snapping/Comp_Anchor Object Reference") (Actor :type "Actor Object Reference") (Connector :type "/XRAIlab/Blueprints/Components/Snapping/Comp_Connector_Anchor Object Reference"))
  (bind _connectorid (`/XRAIlab/Blueprints/Components/Snapping/Comp_Connector_Anchor.ConnectorID` Connector))
  ;[1 1 1] Izquierda
  (if (== _connectorid "L5_1")
    (`BlueprintMapLibrary.Map_Add` (`self.PiezasCorrectas`) _connectorid)
    (`self.Comprobar pieza` :!label _label)))

(event `self.Anchor_5R_1.ActorGotDetached`
  (params (Anchor :type "/XRAIlab/Blueprints/Components/Snapping/Comp_Anchor Object Reference") (Actor :type "Actor Object Reference") (Connector :type "/XRAIlab/Blueprints/Components/Snapping/Comp_Connector_Anchor Object Reference"))
  (bind _connectorid (`/XRAIlab/Blueprints/Components/Snapping/Comp_Connector_Anchor.ConnectorID` Connector))
  ;[1 1 1] Derecha
  (if (== _connectorid "R5_1")
    (`BlueprintMapLibrary.Map_Add` (`self.PiezasCorrectas`) _connectorid)
    (`self.Comprobar pieza` :!label _label_2)))

(event `self.Anchor_5L_1.ActorGotAttached`
  (params (Anchor :type "/XRAIlab/Blueprints/Components/Snapping/Comp_Anchor Object Reference") (Actor :type "Actor Object Reference") (Connector :type "/XRAIlab/Blueprints/Components/Snapping/Comp_Connector_Anchor Object Reference"))
  (bind _connectorid (`/XRAIlab/Blueprints/Components/Snapping/Comp_Connector_Anchor.ConnectorID` Connector))
  ;[1 1 1] Izquierda
  (if (== _connectorid "L5_1")
    (`BlueprintMapLibrary.Map_Add` (`self.PiezasCorrectas`) _connectorid true)
    (`self.Comprobar pieza` :!label _label_3)))

(event `self.Anchor_5R_1.ActorGotAttached`
  (params (Anchor :type "/XRAIlab/Blueprints/Components/Snapping/Comp_Anchor Object Reference") (Actor :type "Actor Object Reference") (Connector :type "/XRAIlab/Blueprints/Components/Snapping/Comp_Connector_Anchor Object Reference"))
  (bind _connectorid (`/XRAIlab/Blueprints/Components/Snapping/Comp_Connector_Anchor.ConnectorID` Connector))
  ;[1 1 1] Derecha
  (if (== _connectorid "R5_1")
    (`BlueprintMapLibrary.Map_Add` (`self.PiezasCorrectas`) _connectorid true)
    (`self.Comprobar pieza` :!label _label_4)))

(event `self.Anchor_5R_2.ActorGotAttached`
  (params (Anchor :type "/XRAIlab/Blueprints/Components/Snapping/Comp_Anchor Object Reference") (Actor :type "Actor Object Reference") (Connector :type "/XRAIlab/Blueprints/Components/Snapping/Comp_Connector_Anchor Object Reference"))
  (bind _connectorid (`/XRAIlab/Blueprints/Components/Snapping/Comp_Connector_Anchor.ConnectorID` Connector))
  ;[1 1 1] Derecha
  (if (== _connectorid "R5_2")
    (`BlueprintMapLibrary.Map_Add` (`self.PiezasCorrectas`) _connectorid true)
    (goto _label_4)))

(event `self.Anchor_5R_2.ActorGotDetached`
  (params (Anchor :type "/XRAIlab/Blueprints/Components/Snapping/Comp_Anchor Object Reference") (Actor :type "Actor Object Reference") (Connector :type "/XRAIlab/Blueprints/Components/Snapping/Comp_Connector_Anchor Object Reference"))
  (bind _connectorid (`/XRAIlab/Blueprints/Components/Snapping/Comp_Connector_Anchor.ConnectorID` Connector))
  ;[1 1 1] Derecha
  (if (== _connectorid "R5_2")
    (`BlueprintMapLibrary.Map_Add` (`self.PiezasCorrectas`) _connectorid)
    (goto _label_2)))

(event `self.Anchor_5L_2.ActorGotDetached`
  (params (Anchor :type "/XRAIlab/Blueprints/Components/Snapping/Comp_Anchor Object Reference") (Actor :type "Actor Object Reference") (Connector :type "/XRAIlab/Blueprints/Components/Snapping/Comp_Connector_Anchor Object Reference"))
  (bind _connectorid (`/XRAIlab/Blueprints/Components/Snapping/Comp_Connector_Anchor.ConnectorID` Connector))
  ;[1 1 1] Izquierda
  (if (== _connectorid "L5_2")
    (`BlueprintMapLibrary.Map_Add` (`self.PiezasCorrectas`) _connectorid)
    (goto _label)))

(event `self.Anchor_5L_2.ActorGotAttached`
  (params (Anchor :type "/XRAIlab/Blueprints/Components/Snapping/Comp_Anchor Object Reference") (Actor :type "Actor Object Reference") (Connector :type "/XRAIlab/Blueprints/Components/Snapping/Comp_Connector_Anchor Object Reference"))
  (bind _connectorid (`/XRAIlab/Blueprints/Components/Snapping/Comp_Connector_Anchor.ConnectorID` Connector))
  ;[1 1 1] Izquierda
  (if (== _connectorid "L5_2")
    (`BlueprintMapLibrary.Map_Add` (`self.PiezasCorrectas`) _connectorid true)
    (goto _label_3)))

(event `self.Anchor_5R_3.ActorGotAttached`
  (params (Anchor :type "/XRAIlab/Blueprints/Components/Snapping/Comp_Anchor Object Reference") (Actor :type "Actor Object Reference") (Connector :type "/XRAIlab/Blueprints/Components/Snapping/Comp_Connector_Anchor Object Reference"))
  (bind _connectorid (`/XRAIlab/Blueprints/Components/Snapping/Comp_Connector_Anchor.ConnectorID` Connector))
  ;[1 1 1] Derecha
  (if (== _connectorid "R5_3")
    (`BlueprintMapLibrary.Map_Add` (`self.PiezasCorrectas`) _connectorid true)
    (goto _label_4)))

(event `self.Anchor_5R_3.ActorGotDetached`
  (params (Anchor :type "/XRAIlab/Blueprints/Components/Snapping/Comp_Anchor Object Reference") (Actor :type "Actor Object Reference") (Connector :type "/XRAIlab/Blueprints/Components/Snapping/Comp_Connector_Anchor Object Reference"))
  (bind _connectorid (`/XRAIlab/Blueprints/Components/Snapping/Comp_Connector_Anchor.ConnectorID` Connector))
  ;[1 1 1] Derecha
  (if (== _connectorid "R5_3")
    (`BlueprintMapLibrary.Map_Add` (`self.PiezasCorrectas`) _connectorid)
    (goto _label_2)))

(event `self.Anchor_5L_3.ActorGotAttached`
  (params (Anchor :type "/XRAIlab/Blueprints/Components/Snapping/Comp_Anchor Object Reference") (Actor :type "Actor Object Reference") (Connector :type "/XRAIlab/Blueprints/Components/Snapping/Comp_Connector_Anchor Object Reference"))
  (bind _connectorid (`/XRAIlab/Blueprints/Components/Snapping/Comp_Connector_Anchor.ConnectorID` Connector))
  ;[1 1 1] Izquierda
  (if (== _connectorid "L5_3")
    (`BlueprintMapLibrary.Map_Add` (`self.PiezasCorrectas`) _connectorid true)
    (goto _label_3)))

(event `self.Anchor_5L_3.ActorGotDetached`
  (params (Anchor :type "/XRAIlab/Blueprints/Components/Snapping/Comp_Anchor Object Reference") (Actor :type "Actor Object Reference") (Connector :type "/XRAIlab/Blueprints/Components/Snapping/Comp_Connector_Anchor Object Reference"))
  (bind _connectorid (`/XRAIlab/Blueprints/Components/Snapping/Comp_Connector_Anchor.ConnectorID` Connector))
  ;[1 1 1] Izquierda
  (if (== _connectorid "L5_3")
    (`BlueprintMapLibrary.Map_Add` (`self.PiezasCorrectas`) _connectorid)
    (goto _label)))

(event `self.Anchor_4R.ActorGotAttached`
  (params (Anchor :type "/XRAIlab/Blueprints/Components/Snapping/Comp_Anchor Object Reference") (Actor :type "Actor Object Reference") (Connector :type "/XRAIlab/Blueprints/Components/Snapping/Comp_Connector_Anchor Object Reference"))
  (bind _connectorid (`/XRAIlab/Blueprints/Components/Snapping/Comp_Connector_Anchor.ConnectorID` Connector))
  ;[1 1 1] Derecha
  (if (== _connectorid "R4")
    (`BlueprintMapLibrary.Map_Add` (`self.PiezasCorrectas`) _connectorid true)
    (goto _label_4)))

(event `self.Anchor_4R.ActorGotDetached`
  (params (Anchor :type "/XRAIlab/Blueprints/Components/Snapping/Comp_Anchor Object Reference") (Actor :type "Actor Object Reference") (Connector :type "/XRAIlab/Blueprints/Components/Snapping/Comp_Connector_Anchor Object Reference"))
  (bind _connectorid (`/XRAIlab/Blueprints/Components/Snapping/Comp_Connector_Anchor.ConnectorID` Connector))
  ;[1 1 1] Derecha
  (if (== _connectorid "R4")
    (`BlueprintMapLibrary.Map_Add` (`self.PiezasCorrectas`) _connectorid)
    (goto _label_2)))

(event `self.Anchor_4L.ActorGotAttached`
  (params (Anchor :type "/XRAIlab/Blueprints/Components/Snapping/Comp_Anchor Object Reference") (Actor :type "Actor Object Reference") (Connector :type "/XRAIlab/Blueprints/Components/Snapping/Comp_Connector_Anchor Object Reference"))
  (bind _connectorid (`/XRAIlab/Blueprints/Components/Snapping/Comp_Connector_Anchor.ConnectorID` Connector))
  ;[1 1 1] Izquierda
  (if (== _connectorid "L4")
    (`BlueprintMapLibrary.Map_Add` (`self.PiezasCorrectas`) _connectorid true)
    (goto _label_3)))

(event `self.Anchor_4L.ActorGotDetached`
  (params (Anchor :type "/XRAIlab/Blueprints/Components/Snapping/Comp_Anchor Object Reference") (Actor :type "Actor Object Reference") (Connector :type "/XRAIlab/Blueprints/Components/Snapping/Comp_Connector_Anchor Object Reference"))
  (bind _connectorid (`/XRAIlab/Blueprints/Components/Snapping/Comp_Connector_Anchor.ConnectorID` Connector))
  ;[1 1 1] Izquierda
  (if (== _connectorid "L4")
    (`BlueprintMapLibrary.Map_Add` (`self.PiezasCorrectas`) _connectorid)
    (goto _label)))

(event `self.Anchor_6R.ActorGotAttached`
  (params (Anchor :type "/XRAIlab/Blueprints/Components/Snapping/Comp_Anchor Object Reference") (Actor :type "Actor Object Reference") (Connector :type "/XRAIlab/Blueprints/Components/Snapping/Comp_Connector_Anchor Object Reference"))
  (bind _connectorid (`/XRAIlab/Blueprints/Components/Snapping/Comp_Connector_Anchor.ConnectorID` Connector))
  ;[1 1 1] Derecha
  (if (== _connectorid "R6")
    (`BlueprintMapLibrary.Map_Add` (`self.PiezasCorrectas`) _connectorid true)
    (goto _label_4)))

(event `self.Anchor_6R.ActorGotDetached`
  (params (Anchor :type "/XRAIlab/Blueprints/Components/Snapping/Comp_Anchor Object Reference") (Actor :type "Actor Object Reference") (Connector :type "/XRAIlab/Blueprints/Components/Snapping/Comp_Connector_Anchor Object Reference"))
  (bind _connectorid (`/XRAIlab/Blueprints/Components/Snapping/Comp_Connector_Anchor.ConnectorID` Connector))
  ;[1 1 1] Derecha
  (if (== _connectorid "R6")
    (`BlueprintMapLibrary.Map_Add` (`self.PiezasCorrectas`) _connectorid)
    (goto _label_2)))

(event `self.Anchor_6L.ActorGotDetached`
  (params (Anchor :type "/XRAIlab/Blueprints/Components/Snapping/Comp_Anchor Object Reference") (Actor :type "Actor Object Reference") (Connector :type "/XRAIlab/Blueprints/Components/Snapping/Comp_Connector_Anchor Object Reference"))
  (bind _connectorid (`/XRAIlab/Blueprints/Components/Snapping/Comp_Connector_Anchor.ConnectorID` Connector))
  ;[1 1 1] Izquierda
  (if (== _connectorid "L6")
    (`BlueprintMapLibrary.Map_Add` (`self.PiezasCorrectas`) _connectorid)
    (goto _label)))

(event `self.Anchor_6L.ActorGotAttached`
  (params (Anchor :type "/XRAIlab/Blueprints/Components/Snapping/Comp_Anchor Object Reference") (Actor :type "Actor Object Reference") (Connector :type "/XRAIlab/Blueprints/Components/Snapping/Comp_Connector_Anchor Object Reference"))
  (bind _connectorid (`/XRAIlab/Blueprints/Components/Snapping/Comp_Connector_Anchor.ConnectorID` Connector))
  ;[1 1 1] Izquierda
  (if (== _connectorid "L6")
    (`BlueprintMapLibrary.Map_Add` (`self.PiezasCorrectas`) _connectorid true)
    (goto _label_3)))

(event `self.Anchor_6R_Fake.ActorGotAttached`
  (params (Anchor :type "/XRAIlab/Blueprints/Components/Snapping/Comp_Anchor Object Reference") (Actor :type "Actor Object Reference") (Connector :type "/XRAIlab/Blueprints/Components/Snapping/Comp_Connector_Anchor Object Reference"))
  ;[1 1 1] Derecha
)

(event `self.Anchor_6R_Fake.ActorGotDetached`
  (params (Anchor :type "/XRAIlab/Blueprints/Components/Snapping/Comp_Anchor Object Reference") (Actor :type "Actor Object Reference") (Connector :type "/XRAIlab/Blueprints/Components/Snapping/Comp_Connector_Anchor Object Reference"))
  ;[1 1 1] Derecha
)

(event `self.Anchor_6L_Fake.ActorGotDetached`
  (params (Anchor :type "/XRAIlab/Blueprints/Components/Snapping/Comp_Anchor Object Reference") (Actor :type "Actor Object Reference") (Connector :type "/XRAIlab/Blueprints/Components/Snapping/Comp_Connector_Anchor Object Reference"))
  ;[1 1 1] Izquierda
)

(event `self.Anchor_6L_Fake.ActorGotAttached`
  (params (Anchor :type "/XRAIlab/Blueprints/Components/Snapping/Comp_Anchor Object Reference") (Actor :type "Actor Object Reference") (Connector :type "/XRAIlab/Blueprints/Components/Snapping/Comp_Connector_Anchor Object Reference"))
  ;[1 1 1] Izquierda
)

(event `self.Anchor_Center.ActorGotAttached`
  (params (Anchor :type "/XRAIlab/Blueprints/Components/Snapping/Comp_Anchor Object Reference") (Actor :type "Actor Object Reference") (Connector :type "/XRAIlab/Blueprints/Components/Snapping/Comp_Connector_Anchor Object Reference"))
  (bind _connectorid (`/XRAIlab/Blueprints/Components/Snapping/Comp_Connector_Anchor.ConnectorID` Connector))
  ;[1 1 1] Center
  (if (== _connectorid "Center")
    (`BlueprintMapLibrary.Map_Add` (`self.PiezasCorrectas`) _connectorid true)
    (`self.Comprobar pieza` :!label _label_5)))

(event `self.Anchor_Center.ActorGotDetached`
  (params (Anchor :type "/XRAIlab/Blueprints/Components/Snapping/Comp_Anchor Object Reference") (Actor :type "Actor Object Reference") (Connector :type "/XRAIlab/Blueprints/Components/Snapping/Comp_Connector_Anchor Object Reference"))
  (bind _connectorid (`/XRAIlab/Blueprints/Components/Snapping/Comp_Connector_Anchor.ConnectorID` Connector))
  ;[1 1 1] Center
  (if (== _connectorid "Center")
    (`BlueprintMapLibrary.Map_Add` (`self.PiezasCorrectas`) _connectorid true)
    (goto _label_5)))

(event `Comprobar pieza`
  (bind _anchortomeshmap (`self.AnchorToMeshMap`))
  ;[1 1 1] Boton
  (if (== (`BlueprintMapLibrary.Map_Length` (`self.PiezasCorrectas`)) 12)
    (`/Game/TFG/BP/BP_Oña_GameStateBase.ChangeGamePhase` (`self.As BP Oña Game State Base`) "NewEnumerator3")
    (else
      (`KismetSystemLibrary.Delay` 1.0)
      (bind _keys (`BlueprintMapLibrary.Map_Keys` _anchortomeshmap))
      (for _array_element _keys
        (if (`BlueprintMapLibrary.Map_Find` (`self.PiezasCorrectas`) _array_element)
          (bind _value (`BlueprintMapLibrary.Map_Find` _anchortomeshmap _array_element))
          (`self.SetActorHiddenInGame` _value false)
          (else
            (`self.SetActorHiddenInGame` _value true)))))))

(fn `UserConstructionScript`)