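; VR game state for the Oña experience that runs Setup, narrated intro, timed gameplay and narrated outro phases.
; BeginPlay caches tagged environment, board and piece actors plus the crafting table, then enters Setup, which hides them.
; Each phase toggles their visibility; the intro, triggered externally, also resets headset orientation.
; Audio-finished callbacks and a one-second countdown timer advance later phases, ending by opening Map_Template.
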(event `self.ReceiveBeginPlay`
  (`|ExecutionSequence`
    (:`then_0`
      (bind _outactors (`GameplayStatics.GetAllActorsWithTag` "Env"))
      (set `self.RefEnv` _outactors))
    (:`then_1`
      (bind _outactors_2 (`GameplayStatics.GetAllActorsWithTag` "Tabla"))
      (set `self.RefTabla` _outactors_2))
    (:`then_2`
      (bind _outactors_3 (`GameplayStatics.GetAllActorsWithTag` "Pieza"))
      (set `self.Piezas` _outactors_3))
    (:`then_3`
      (bind _returnvalue (`GameplayStatics.GetActorOfClass` "/Game/TFG/BP/BP_CraftingTable.BP_CraftingTable_C"))
      (set `self.RefMesa` _returnvalue))
    (:`then_4`
      (bind _returnvalue_2 (`GameplayStatics.GetActorOfClass` "/XRAIlab/Blueprints/Pawn/VR/BP_Pawn_VR.BP_Pawn_VR_C"))
      (set `self.RefPlayer` _returnvalue_2))
    (:`then_5`
      (`self.ChangeGamePhase` "NewEnumerator0"))))

(event `ChangeGamePhase`
  (params (NewPhase :type "/Game/TFG/BP/E_GamePhase Enum" :default "NewEnumerator0"))
  (bind _output_get (set `self.CurrentPhase ` NewPhase))
  (switch `/Game/TFG/BP/E_GamePhase` _output_get
    (:`NewEnumerator0`
      (`self.Event_Phase_Setup`))
    (:`NewEnumerator1`
      (`self.Event_Phase_AudioIntro`))
    (:`NewEnumerator2`
      (`self.Event_Phase_Gameplay`))
    (:`NewEnumerator3`
      (`self.Event_Phase_AudioOutro`))))

(event `Event_Phase_Setup`
  (`KismetSystemLibrary.PrintString` "Setup start")
  (`self.DesactivarArrary` true (`self.Piezas`))
  (`self.DesactivarArrary` true (`self.RefEnv`))
  (`self.DesactivarArrary` true (`self.RefTabla`))
  (`self.SetActorHiddenInGame` (`self.RefMesa`) true))

(event `Event_Phase_AudioIntro`
  (`KismetSystemLibrary.PrintString` "Audio start")
  (`self.ResetRotation`)
  (`self.DesactivarArrary` false (`self.RefEnv`))
  (bind _returnvalue (`GameplayStatics.SpawnSound2D` "/Game/TFG/ASSETS/AUD/AUD_NarracionInicio.AUD_NarracionInicio" 1.0 1.0 0.0 null false false))
  (add `AudioComponent.OnAudioFinished` _returnvalue (delegate `OnIntroAudioFinished`)))

(event `OnIntroAudioFinished`
  (`ActorComponent.K2_DestroyComponent` (stale `Event_Phase_AudioIntro` _returnvalue))
  (`self.ChangeGamePhase` "NewEnumerator2"))

(event `Event_Phase_Gameplay`
  (`KismetSystemLibrary.PrintString` "Game start")
  (`self.DesactivarArrary` false (`self.Piezas`))
  (`self.SetActorHiddenInGame` (`self.RefMesa`) false)
  (bind _returnvalue (`KismetSystemLibrary.K2_SetTimerDelegate` (delegate `Tick_Reloj`) 1.0 true))
  (bind _output_get (set `self.Temporizador_Handle ` _returnvalue)))

(event `Tick_Reloj`
  (bind _result (`/Engine/EditorBlueprintResources/StandardMacros.DecrementFloat` (`self.TiempoRestante `))
    (:`  `
      (bind _output_get (set `self.TiempoRestante ` _result))
      (if (<= _output_get 0.0)
        (`KismetSystemLibrary.K2_ClearAndInvalidateTimerHandle` (stale `Event_Phase_Gameplay` _output_get))
        (`self.ChangeGamePhase` "NewEnumerator3")))))

(event `Event_Phase_AudioOutro`
  (`KismetSystemLibrary.PrintString` "Audio 2 start")
  (`self.DesactivarArrary` true (`self.Piezas`))
  (`self.SetActorHiddenInGame` (`self.RefMesa`) true)
  (`self.DesactivarArrary` false (`self.RefTabla`))
  (bind _returnvalue (`GameplayStatics.SpawnSound2D` "/Game/TFG/ASSETS/AUD/AUD_NarracionFinal.AUD_NarracionFinal" 1.0 1.0 0.0 null false false))
  (add `AudioComponent.OnAudioFinished` _returnvalue (delegate `OnOutroAudioFInished`)))

(event `OnOutroAudioFInished`
  (`KismetSystemLibrary.Delay` 2.0)
  (`GameplayStatics.OpenLevel` "Map_Template")
  (`self.ChangeGamePhase` "NewEnumerator0"))

(event `ResetRotation`
  (bind (_returnvalue_roll _returnvalue_pitch _returnvalue_yaw) (`KismetMathLibrary.BreakRotator` (`KismetMathLibrary.FindLookAtRotation` (`self.K2_GetActorLocation`) (`self.K2_GetActorLocation` (`GameplayStatics.GetPlayerCharacter` 0)))))
  (`HeadMountedDisplayFunctionLibrary.ResetOrientationAndPosition` _returnvalue_yaw))

(event `DesactivarArrary`
  (params (`Desactivar piezas` :type Boolean) (Array :type "Array of Actor Object Reference"))
  (for _array_element Array
    (`self.SetActorHiddenInGame` _array_element `Desactivar piezas`)))

(fn `UserConstructionScript`)